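; AnthroGameMode is the game mode that runs a turn-based, multi-player round structure with per-turn action points.
; NextPlayer refills action points and advances the active player up to GlobalData's player count, calling next-turn, then wraps to end and restart the round and increments the turn count.
; Player stat objects are stored in an array indexed by player number for active-player lookup.
; CheckAP tests the requested cost but always deducts just one point on success.
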(event `self.ReceiveBeginPlay`
  (set `self.activePlayer` "PN_0")
  (set `self.actionPoints` (`self.maxAP`)))

(fn `AddPlayer`
  (params (playerStats :type "/Game/Blueprints/Gameplay/PlayerStatsMain Object Reference"))
  (`KismetArrayLibrary.Array_Set` (`self.PlayerStatObjects`) (`KismetMathLibrary.Conv_ByteToInt` (`/Game/Blueprints/Gameplay/PlayerStatsMain.playerNo` playerStats)) playerStats true))

(fn `CheckAP`
  (params (DecreaseAP :type Integer))
  (returns (isEnoughAP :type Boolean))
  (bind _actionpoints (`self.actionPoints`))
  (if (>= (`self.actionPoints`) DecreaseAP)
    (set `self.actionPoints` (- _actionpoints 1))
    (`KismetSystemLibrary.PrintString` (`KismetStringLibrary.Concat_StrStr` (`KismetStringLibrary.Conv_IntToString` _actionpoints) " action left"))
    (return true)
    (else
      (`KismetSystemLibrary.PrintString` "NotEnoughActionPoints")
      (return false))))

(fn `Get Active Player`
  (returns (Output :type "/Game/Blueprints/Gameplay/PlayerStatsMain Object Reference") (enumOutput :type "EPlayerNo Enum"))
  (bind _activeplayer (`self.activePlayer`))
  (return (`KismetArrayLibrary.Array_Get` (`self.PlayerStatObjects`) (`KismetMathLibrary.Conv_ByteToInt` _activeplayer)) _activeplayer))

(fn `nextPlayer`
  (set `self.actionPoints` (`self.maxAP`))
  (bind _output_get (set `self.activePlayer` (cast `EPlayerNo` (+ (`self.activePlayer`) 1))))
  (bind _asglobal_data (cast `/Game/Blueprints/Gameplay/GlobalData` (`GameplayStatics.GetGameInstance`)))
  (if (< _output_get (`/Game/Blueprints/Gameplay/GlobalData.NumberOfPlayers` _asglobal_data))
    (`KismetSystemLibrary.PrintString` "next player")
    (`self.NextTurn`)
    (else
      (set `self.activePlayer` "PN_0")
      (`self.EndRound`)
      (`KismetSystemLibrary.PrintString` "End Round" false)
      (`/Engine/EditorBlueprintResources/StandardMacros.IncrementInt` (`self.TurnCount`)
        (:`  `
          (`self.StartRound`))))))

(fn `UserConstructionScript`)