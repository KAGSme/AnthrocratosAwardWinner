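; Editor camera pawn that pans, orbits and zooms, and also handles pause-menu toggling and returning to the main menu.
; Tick pushes a physics Box from held movement keys or screen-edge cursor position, with a looping MultiGate checking one direction per frame.
; Holding Confirm drags the camera, while Extra or the Rotate axis strafes and re-aims yaw at MainController's active tile or a point ahead.
; Zoom adjusts clamped FOV, and position clamping is optional.
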(event EventTick
  (params (DeltaSeconds :type Float%20%28single-precision%29))
  (bind _returnvalue (Viewport|GetViewportSize))
  (bind _returnvalue_2 (Viewport|GetViewportSize))
  (bind _returnvalue_3 (Game|GetPlayerController 0))
  (bind _moveoncursor (Variables|Default|GetMoveOnCursor))
  (bind _rotateoncursor (Variables|Default|GetRotateOnCursor))
  (bind _margin (Variables|Default|Getmargin))
  (bind (_locationx _locationy) (Game|Player|GetMousePosition _returnvalue_3))
  (bind (_x _y) (Math|Vector2D|BreakVector2D _returnvalue))
  (bind (_x_2 _y_2) (Math|Vector2D|BreakVector2D _returnvalue_2))
  (bind _returnvalue_4 (- 1.0 _margin))
  (if (Game|IsGamePaused)
    (Variables|Default|SetAHeld false)
    (Variables|Default|SetSHeld false)
    (Variables|Default|SetDHeld false)
    (Variables|Default|SetWHeld false))
  (bind _aseditor_controller (Utilities|Casting|CastToEditorController (Game|GetPlayerController 0)))
  (if _rotateoncursor
    (CallFunction|Rotate (Class|Actor|GetInputAxisKeyValue)))
  (CallFunction|MovebyCursor _moveoncursor)
  (CallFunction|LockPosition (Variables|Default|GetLockMaxX) (Variables|Default|GetLockMaxY))
  (if (and (not _rotateoncursor) (not _moveoncursor))
    (Variables|/Script/Engine.PlayerController|SetbShowMouseCursor _aseditor_controller true)
    (Variables|Default|SetMoveX (Math|Transform|TransformDirection (Transformation|GetActorTransform self) "1.000000, 0, 0"))
    (Variables|Default|SetMoveY (Math|Transform|TransformDirection (Transformation|GetActorTransform self) "0.000000,1.000000, 0"))
    (Variables|/Script/Engine.PlayerController|SetbShowMouseCursor _returnvalue_3 true)
    (Utilities|FlowControl|MultiGate false true -1
      (:Out%200
        ;[1 1 1] Camera Movement
        (if (or (Variables|Default|GetAHeld) (<= _locationx (* _x_2 _margin)))
          (Physics|AddImpulse (Variables|Default|GetBox) (* (* (Variables|Default|GetMoveY) -1) (Variables|Default|GetVelocity)) "None" false)))
      (:Out%201
        (if (or (Variables|Default|GetDHeld) (>= _locationx (* _x _returnvalue_4)))
          (Physics|AddImpulse (Variables|Default|GetBox) (* (Variables|Default|GetMoveY) (Variables|Default|GetVelocity)) "None" false)))
      (:Out%202
        (if (or (Variables|Default|GetSHeld) (>= _locationy (* _y _returnvalue_4)))
          (Physics|AddImpulse (Variables|Default|GetBox) (* (* (Variables|Default|GetMoveX) -1) (Variables|Default|GetVelocity)) "None" false)))
      (:Out%203
        (if (or (<= _locationy (* _y_2 _margin)) (Variables|Default|GetWHeld))
          (Physics|AddImpulse (Variables|Default|GetBox) (* (Variables|Default|GetMoveX) (Variables|Default|GetVelocity)) "None" false))))
    (else
      (Variables|/Script/Engine.PlayerController|SetbShowMouseCursor _aseditor_controller false))))

(event EventBeginPlay
  (bind _aseditor_controller (Utilities|Casting|CastToEditorController (Game|GetPlayerController 0)))
  (Input|SetInputModeGameandUI (Game|GetPlayerController 0) (Variables|/Game/Blueprints/Gameplay/EditorController.EditorController_C|GetEditorUIRef _aseditor_controller) true false))

(event Input|ActionEvents|InputActionExtra
  (params (Key :type Key%20Structure :default "AnyKey"))
  (:Pressed
    (Variables|Default|SetRotateOnCursor true))
  (:Released
    (Variables|Default|SetRotateOnCursor false)))

(event Input|ActionEvents|InputActionUpMovement
  (params (Key :type Key%20Structure :default "AnyKey"))
  ;[1 1 1] Keyboard Movement (Maybe this won't be needed if camera is fixed)
  (:Pressed
    (Variables|Default|SetWHeld true))
  (:Released
    (Variables|Default|SetWHeld false)))

(event Input|ActionEvents|InputActionLeftMovement
  (params (Key :type Key%20Structure :default "AnyKey"))
  ;[1 1 1] Keyboard Movement (Maybe this won't be needed if camera is fixed)
  (:Pressed
    (Variables|Default|SetAHeld true))
  (:Released
    (Variables|Default|SetAHeld false)))

(event Input|ActionEvents|InputActionDownMovement
  (params (Key :type Key%20Structure :default "AnyKey"))
  ;[1 1 1] Keyboard Movement (Maybe this won't be needed if camera is fixed)
  (:Pressed
    (Variables|Default|SetSHeld true))
  (:Released
    (Variables|Default|SetSHeld false)))

(event Input|ActionEvents|InputActionRightMovement
  (params (Key :type Key%20Structure :default "AnyKey"))
  ;[1 1 1] Keyboard Movement (Maybe this won't be needed if camera is fixed)
  (:Pressed
    (Variables|Default|SetDHeld true))
  (:Released
    (Variables|Default|SetDHeld false)))

(event Input|ActionEvents|InputActionConfirm
  (params (Key :type Key%20Structure :default "AnyKey"))
  (:Pressed
    (Variables|Default|SetMoveOnCursor true))
  (:Released
    (Variables|Default|SetMoveOnCursor false)))

(event Input|AxisEvents|InputAxisRotate
  (params (AxisValue :type Float%20%28single-precision%29))
  (CallFunction|Rotate AxisValue))

(event Input|AxisEvents|InputAxisZoom
  (params (AxisValue :type Float%20%28single-precision%29))
  (CallFunction|Zoom AxisValue))

(event Input|KeyboardEvents|Backspace
  (params (Key :type Key%20Structure :default "AnyKey"))
  (:Pressed
    (Game|OpenLevel(byName) "MainMenu")))

(event Input|KeyboardEvents|M
  (params (Key :type Key%20Structure :default "AnyKey"))
  (:Pressed
    (bind _aseditor_controller (Utilities|Casting|CastToEditorController (Game|GetPlayerController 0)))
    (if (Widget|IsVisible (Variables|/Game/Blueprints/Gameplay/EditorController.EditorController_C|GetPauseMenuRef _aseditor_controller))
      (Widget|SetVisibility (Variables|/Game/Blueprints/Gameplay/EditorController.EditorController_C|GetPauseMenuRef _aseditor_controller) "Hidden")
      (Widget|SetVisibility (Variables|/Game/Blueprints/UI/PauseMenu.PauseMenu_C|GetOptionsBox (Variables|/Game/Blueprints/Gameplay/EditorController.EditorController_C|GetPauseMenuRef _aseditor_controller)) "Hidden")
      (Game|SetGamePaused false)
      (else
        (Widget|SetVisibility (Variables|/Game/Blueprints/Gameplay/EditorController.EditorController_C|GetPauseMenuRef _aseditor_controller) "Visible")
        (Game|SetGamePaused true)))))

(fn ConstructionScript)

(fn Zoom
  (params (Direction :type Float%20%28single-precision%29))
  (bind _camera (Variables|Default|GetCamera))
  (Variables|/Script/Engine.CameraComponent|SetFieldOfView _camera (Math|Float|Clamp(Float) (+ (* Direction 1e+01) (Variables|/Script/Engine.CameraComponent|GetFieldOfView _camera)) 3e+01 1.1e+02)))

(fn Rotate
  (params (Direction :type Float%20%28single-precision%29))
  (bind _returnvalue (Transformation|GetActorRotation))
  (if (!= Direction 0.0)
    (bind _asmain_controller (Utilities|Casting|CastToMainController (Game|GetPlayerController 0)))
    (if (!= (Variables|/Game/Blueprints/Gameplay/MainController.MainController_C|GetActiveTile _asmain_controller) 0)
      (LocalVariables|SetTarget (Transformation|GetActorLocation (Variables|/Game/Blueprints/Gameplay/MainController.MainController_C|GetActiveTile _asmain_controller)))
      (else
        (LocalVariables|SetTarget (+ (* (Math|Vector|Normalize (Math|Vector|GetForwardVector (Transformation|GetActorRotation))) "100.000000,100.000000,100.000000") (Transformation|GetActorLocation)))))
    (Transformation|AddActorWorldOffset (* (Variables|Default|GetMoveY) (* (Variables|Default|GetRotationVelocity) Direction)))
    (Transformation|SetActorRelativeRotation (Math|Rotator|MakeRotator (.roll _returnvalue) (.pitch _returnvalue) (.Yaw (Math|Rotator|BreakRotator (Math|Rotator|FindLookatRotation (Transformation|GetActorLocation) (LocalVariables|GetTarget))))))))

(fn LockPosition
  (params (X :type Float%20%28single-precision%29) (Y :type Float%20%28single-precision%29))
  (bind _returnvalue (Transformation|GetActorLocation))
  ;[1 1 1] Old
  (if (Variables|Default|GetClampPosition)
    (Transformation|SetActorLocation (Math|Vector|MakeVector (Math|Float|Clamp(Float) (.x _returnvalue) -2e+01 X) (Math|Float|Clamp(Float) (.y _returnvalue) -2e+01 Y) (.z _returnvalue)) false true)))

(fn BorderMovement)

(fn MovebyCursor
  (params (MoveOnCursor :type Boolean))
  (bind _movebycursorspeed (Variables|Default|GetMoveByCursorSpeed))
  (if MoveOnCursor
    (Transformation|SetActorLocation (+ (Transformation|GetActorLocation) (* (Variables|Default|GetMoveX) (* (Class|Actor|GetInputAxisKeyValue) _movebycursorspeed -1.0)) (* (Variables|Default|GetMoveY) (* (Class|Actor|GetInputAxisKeyValue) _movebycursorspeed -1.0))) false false)))