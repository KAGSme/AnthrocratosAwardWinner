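; Main controller that creates the game's UI widgets on BeginPlay, tracks the selected tile and handles notifications and saving.
; Notifications go into a scrollable log plus a temporary HUD copy that a timeline fades out and clears.
; The tile interaction panel gets one entry per BuildingsData row, showing biome bonuses.
; SaveGame stores two players' resources in one slot; LoadGame only prints saved values, without restoring them.
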(event `self.ReceiveBeginPlay`
  (bind _returnvalue (`|CreateWidget` "/Game/Blueprints/UI/HUD_Main.HUD_Main_C"))
  (set `self.HUDMainRef` _returnvalue)
  (`UserWidget.AddToViewport` _returnvalue 1)
  (bind _returnvalue_2 (`|CreateWidget` "/Game/Blueprints/UI/UpgradeBuildingUI.UpgradeBuildingUI_C"))
  (set `self.UpgradeUIRef` _returnvalue_2)
  (`UserWidget.AddToViewport` _returnvalue_2 6)
  (bind _returnvalue_3 (`|CreateWidget` "/Game/Blueprints/UI/NotificationUI.NotificationUI_C"))
  (set `self.NotificationRef` _returnvalue_3)
  (bind _returnvalue_4 (`|CreateWidget` "/Game/Blueprints/UI/NextPlayer.NextPlayer_C"))
  (`UserWidget.AddToViewport` _returnvalue_3 8)
  (`UserWidget.AddToViewport` _returnvalue_4 8)
  (`Widget.SetVisibility` _returnvalue_3 "Hidden")
  (`Widget.SetVisibility` _returnvalue_2 "Hidden")
  (`Widget.SetVisibility` _returnvalue_4 "Hidden")
  (bind _returnvalue_5 (`|CreateWidget` "/Game/Blueprints/UI/TileInteractionUI.TileInteractionUI_C"))
  (set `self.TileInteractionRef` _returnvalue_5)
  (`UserWidget.AddToViewport` _returnvalue_5 6)
  (bind _returnvalue_6 (`|CreateWidget` "/Game/Blueprints/UI/PauseMenu.PauseMenu_C"))
  (set `self.PauseMenuRef` _returnvalue_6)
  (`UserWidget.AddToViewport` _returnvalue_6 6)
  (`self.AddInteraction`))

(event `FadeNotification`
  (params (Notification :type "Button Object Reference"))
  (bind (_direction _alphavalues) (`Timeline|FadeTimeline` :!via `PlayFromStart`)
    (:`Update`
      (`Button.SetColorAndOpacity` Notification (`KismetMathLibrary.MakeColor` 0.0 0.0 0.0 _alphavalues)))
    (:`Finished`
      (`PanelWidget.ClearChildren` (`/Game/Blueprints/UI/HUD_Main.TempNotification` (`self.HUDMainRef`)))
      (`/Engine/EditorBlueprintResources/StandardMacros.DecrementInt` (`self.NoOfNotications`)))))

(fn `AddInteraction`
  (bind _outrownames (`DataTableFunctionLibrary.GetDataTableRowNames` "/Game/Blueprints/Tiles/Buildings/BuildingsData.BuildingsData"))
  (for _array_element _outrownames
    (bind _createdinteraction (`self.CreateInteraction` _array_element))
    (`PanelWidget.AddChild` (`/Game/Blueprints/UI/TileInteractionUI.InteractionScrollBox` (`self.TileInteractionRef`)) _createdinteraction)))

(fn `AddNotification`
  (params (NotificationText :type String))
  (bind _tempnotification (`/Game/Blueprints/UI/HUD_Main.TempNotification` (`self.HUDMainRef`)))
  (bind _creatednotification (`self.CreateNotification` NotificationText))
  (`PanelWidget.AddChild` (`/Game/Blueprints/UI/NotificationUI.NotificationScrollBox` (`self.NotificationRef`)) _creatednotification)
  (`Button.SetColorAndOpacity` _creatednotification (struct :`A` 1.0))
  (bind _creatednotification_2 (`self.CreateNotification` NotificationText))
  (`PanelWidget.ClearChildren` _tempnotification)
  (`PanelWidget.AddChild` _tempnotification _creatednotification_2)
  (`self.FadeNotification` _creatednotification_2))

(fn `CreateInteraction`
  (params (RowNumber :type Name))
  (returns (CreatedInteraction :type "Button Object Reference"))
  (bind _returnvalue (`|GetDataTableRow` "/Game/Blueprints/Tiles/Buildings/BuildingsData.BuildingsData" RowNumber)
    (:`then`
      (bind _returnvalue_2 (`|CreateWidget` "/Game/Blueprints/UI/SingleInteraction.SingleInteraction_C" (`GameplayStatics.GetPlayerController` 0)))
      (bind (_moneycost _foodcost _energycost _moneyupkeep _foodupkeep _energyupkeep _moneygenerated _foodgenerated _energygenerated _happinessgenerated _biomebonus _biomebonuseffect) (break `/Game/Blueprints/Tiles/Buildings/BuildingsDataStructure` _returnvalue))
      (`TextBlock.SetText` (`/Game/Blueprints/UI/SingleInteraction.Biome1` _returnvalue_2) (`KismetTextLibrary.Conv_StringToText` (`|GetEnumeratorNameAsString` (`KismetArrayLibrary.Array_Get` _biomebonus))))
      (bind _item (`KismetArrayLibrary.Array_Get` _biomebonuseffect))
      (if (> _item 0)
        (bind _biome1effect (`/Game/Blueprints/UI/SingleInteraction.Biome1Effect` _returnvalue_2))
        (bind _returnvalue_3 (`KismetTextLibrary.Conv_IntToText` _item))
        (`TextBlock.SetText` _biome1effect (`KismetTextLibrary.Conv_StringToText` (`KismetStringLibrary.Concat_StrStr` "+" (`KismetTextLibrary.Conv_TextToString` _returnvalue_3))))
        (else
          (`TextBlock.SetText` _biome1effect _returnvalue_3)))
      (`TextBlock.SetText` (`/Game/Blueprints/UI/SingleInteraction.Biome2` _returnvalue_2) (`KismetTextLibrary.Conv_StringToText` (`|GetEnumeratorNameAsString` (`KismetArrayLibrary.Array_Get` _biomebonus 1))))
      (bind _item_2 (`KismetArrayLibrary.Array_Get` _biomebonuseffect 1))
      (if (> _item_2 0)
        (bind _biome2effect (`/Game/Blueprints/UI/SingleInteraction.Biome2Effect` _returnvalue_2))
        (bind _returnvalue_4 (`KismetTextLibrary.Conv_IntToText` _item_2))
        (`TextBlock.SetText` _biome2effect (`KismetTextLibrary.Conv_StringToText` (`KismetStringLibrary.Concat_StrStr` "+" (`KismetTextLibrary.Conv_TextToString` _returnvalue_4))))
        (else
          (`TextBlock.SetText` _biome2effect _returnvalue_4)))
      (`TextBlock.SetText` (`/Game/Blueprints/UI/SingleInteraction.BuildingName` _returnvalue_2) (`KismetTextLibrary.Conv_NameToText` RowNumber))
      (return (`/Game/Blueprints/UI/SingleInteraction.InteractionOutline` _returnvalue_2)))
    (:`RowNotFound`
      (return null))))

(fn `CreateNotification`
  (params (NotificationText :type String))
  (returns (CreatedNotification :type "Button Object Reference"))
  (bind _returnvalue (`|CreateWidget` "/Game/Blueprints/UI/SingleNotification.SingleNotification_C" (`GameplayStatics.GetPlayerController` 0)))
  (set `/Game/Blueprints/UI/SingleNotification.ThisNotification` NotificationText _returnvalue)
  (`TextBlock.SetText` (`/Game/Blueprints/UI/SingleNotification.NotificationText` _returnvalue) (`KismetTextLibrary.Conv_StringToText` NotificationText))
  (return (`/Game/Blueprints/UI/SingleNotification.NotificationOutline` _returnvalue)))

(fn `GetSelectedTile`
  (returns (SelectedTile :type "/Game/Blueprints/Tiles/Biomes/HexTileBasic Object Reference"))
  (return (`self.ActiveTile`)))

(fn `LoadGame`
  (bind _returnvalue (`GameplayStatics.DoesSaveGameExist` "Save1"))
  (if _returnvalue
    (bind _returnvalue_2 (`GameplayStatics.LoadGameFromSlot` "Save1"))
    (bind _asanthro_save_game (cast `/Game/Blueprints/Gameplay/AnthroSaveGame` _returnvalue_2))
    (bind _output_get (set `self.SaveGameState` _asanthro_save_game))
    (`KismetSystemLibrary.PrintString` (`KismetStringLibrary.Concat_StrStr` "Player1: Money" (`KismetStringLibrary.Conv_IntToString` (`/Game/Blueprints/Gameplay/AnthroSaveGame.p1Money` _output_get)) "Food: " (`KismetStringLibrary.Conv_IntToString` (`/Game/Blueprints/Gameplay/AnthroSaveGame.p1Food` _output_get)) "Energy: " (`KismetStringLibrary.Conv_IntToString` (`/Game/Blueprints/Gameplay/AnthroSaveGame.p1Energy` _output_get)) "Player 2: Money" (`KismetStringLibrary.Conv_IntToString` (`/Game/Blueprints/Gameplay/AnthroSaveGame.p2Money` _output_get)) "Food: " (`KismetStringLibrary.Conv_IntToString` (`/Game/Blueprints/Gameplay/AnthroSaveGame.p2Food` _output_get)) "Energy: " (`KismetStringLibrary.Conv_IntToString` (`/Game/Blueprints/Gameplay/AnthroSaveGame.p2Energy` _output_get))))
    (else
      (`KismetSystemLibrary.PrintString` "No save data"))))

(fn `SaveGame`
  (bind _returnvalue (`GameplayStatics.CreateSaveGameObject` "/Game/Blueprints/Gameplay/AnthroSaveGame.AnthroSaveGame_C"))
  (bind _asanthro_save_game (cast `/Game/Blueprints/Gameplay/AnthroSaveGame` _returnvalue))
  (bind _output_get (set `self.SaveGameState` _asanthro_save_game))
  (bind _outactors (`GameplayStatics.GetAllActorsOfClass` "/Game/Blueprints/Gameplay/PlayerStatsMain.PlayerStatsMain_C"))
  (bind _item (`KismetArrayLibrary.Array_Get` _outactors))
  (set `/Game/Blueprints/Gameplay/AnthroSaveGame.p1Money` (`/Game/Blueprints/Gameplay/PlayerStatsMain.Money` _item) _output_get)
  (set `/Game/Blueprints/Gameplay/AnthroSaveGame.p1Food` (`/Game/Blueprints/Gameplay/PlayerStatsMain.Food` _item) _output_get)
  (set `/Game/Blueprints/Gameplay/AnthroSaveGame.p1Energy` (`/Game/Blueprints/Gameplay/PlayerStatsMain.Energy` _item) _output_get)
  (set `/Game/Blueprints/Gameplay/AnthroSaveGame.p1Happiness` (`/Game/Blueprints/Gameplay/PlayerStatsMain.Happiness` _item) _output_get)
  (bind _item_2 (`KismetArrayLibrary.Array_Get` _outactors 1))
  (set `/Game/Blueprints/Gameplay/AnthroSaveGame.p2Money` (`/Game/Blueprints/Gameplay/PlayerStatsMain.Money` _item_2) _output_get)
  (set `/Game/Blueprints/Gameplay/AnthroSaveGame.p2Food` (`/Game/Blueprints/Gameplay/PlayerStatsMain.Food` _item_2) _output_get)
  (set `/Game/Blueprints/Gameplay/AnthroSaveGame.p2Energy` (`/Game/Blueprints/Gameplay/PlayerStatsMain.Energy` _item_2) _output_get)
  (set `/Game/Blueprints/Gameplay/AnthroSaveGame.p2Happiness` (`/Game/Blueprints/Gameplay/PlayerStatsMain.Happiness` _item_2) _output_get)
  (`GameplayStatics.SaveGameToSlot` (`self.SaveGameState`) "Save1"))

(fn `SetSelectedTile`
  (params (`new tile` :type "/Game/Blueprints/Tiles/Biomes/HexTileBasic Object Reference"))
  (returns (Output :type "/Game/Blueprints/Tiles/Biomes/HexTileBasic Object Reference"))
  (bind _output_get (set `self.ActiveTile` `new tile`))
  (return _output_get))

(fn `UserConstructionScript`)