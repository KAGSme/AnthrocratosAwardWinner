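; Per-player state for a turn-based hex-tile building game, holding resources, Happiness, owned buildings and spawnable building types.
; It registers with AnthroGameMode, whose round start triggers a Happiness win check, adds base funding and clamps negative Happiness.
; AttemptSpawnBuilding spawns the building first, then destroys it if resource or action-point checks fail, otherwise charging, tracking and player-tinting it.
; GetGeneration totals funding, building output, upkeep and biome bonuses.
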(event `/Game/Blueprints/Gameplay/iStatsAndFlows.TrackBuilding`
  (params (Building :type "/Game/Blueprints/Tiles/Buildings/Building Object Reference"))
  (`KismetArrayLibrary.Array_AddUnique` (`self.BuildingsOwned`) Building)
  (`KismetSystemLibrary.PrintString` "BuildingTracked" false))

(event `/Game/Blueprints/Gameplay/iStatsAndFlows.UntrackBuilding`
  (params (Building :type "/Game/Blueprints/Tiles/Buildings/Building Object Reference"))
  (bind _returnvalue (`KismetArrayLibrary.Array_RemoveItem` (`self.BuildingsOwned`) Building))
  (if _returnvalue
    (`KismetSystemLibrary.PrintString` "BuildingUntracked" false)))

(event `/Game/Blueprints/Gameplay/iStatsAndFlows.AddEnergy`
  (params (Energy :type Integer))
  (set `self.Energy` (+ Energy (`self.Energy`))))

(event `/Game/Blueprints/Gameplay/iStatsAndFlows.AddFood`
  (params (Food :type Integer))
  (set `self.Food` (+ Food (`self.Food`))))

(event `/Game/Blueprints/Gameplay/iStatsAndFlows.AddHappiness`
  (params (Happiness :type Integer))
  (set `self.Happiness` (+ Happiness (`self.Happiness`))))

(event `/Game/Blueprints/Gameplay/iStatsAndFlows.AddMoney `
  (params (MoneyAdded :type Integer))
  (set `self.Money` (+ MoneyAdded (`self.Money`))))

(event `self.ReceiveBeginPlay`
  (bind _asanthro_game_mode (cast `/Game/Blueprints/Gamemodes/AnthroGameMode` (`GameplayStatics.GetGameMode`)))
  (`/Game/Blueprints/Gamemodes/AnthroGameMode.AddPlayer` _asanthro_game_mode self)
  (add `/Game/Blueprints/Gamemodes/AnthroGameMode.StartRound` _asanthro_game_mode (delegate `StartRoundCall`)))

(event `StartRoundCall`
  (`self.CheckWinConditions`)
  (`self.AddFunding`)
  (if (< (`self.Happiness`) 0)
    (set `self.Happiness` 0)))

(fn `AddBuildingType`
  (params (BuildingType :type "/Game/Blueprints/Tiles/Buildings/Building Class Reference") (Money :type Integer) (Food :type Integer) (Energy :type Integer))
  (bind _spawnablebuildings (`self.SpawnableBuildings`))
  (if (`KismetArrayLibrary.Array_Contains` _spawnablebuildings BuildingType)
    (`KismetSystemLibrary.PrintString` "PlayerAlreadyHasBuilding")
    (else
      (`KismetArrayLibrary.Array_AddUnique` _spawnablebuildings BuildingType))))

(fn `AddFunding`
  (bind _funding (`self.Funding`))
  (`self.AddMoney ` _funding)
  (`self.AddFood` _funding)
  (`self.AddEnergy` _funding))

(fn `AttemptSpawnBuilding`
  (params (BuildingToSpawn :type "/Game/Blueprints/Tiles/Buildings/Building Class Reference (by ref)") (HexTileRef :type "/Game/Blueprints/Tiles/Biomes/HexTileBasic Object Reference (by ref)"))
  (returns (isSuccessful :type Boolean) (Location :type "Transform Structure") (Building :type "/Game/Blueprints/Tiles/Buildings/Building Object Reference"))
  (bind _returnvalue (`KismetMathLibrary.MakeTransform` (`/Game/Blueprints/Tiles/Biomes/HexTileBasic.TilePosition` HexTileRef) (struct) (1.0 1.0 1.0)))
  (if (!= HexTileRef null)
    (bind _asanthro_game_mode (cast `/Game/Blueprints/Gamemodes/AnthroGameMode` (`GameplayStatics.GetGameMode`))
      (:`then`
        (bind _returnvalue_2 (`|SpawnActorFromClass` BuildingToSpawn _returnvalue "Undefined" "OverrideRootScale"))
        (bind _isenough (`self.CheckResources` (`/Game/Blueprints/Tiles/Buildings/Building.money_cost` _returnvalue_2) (`/Game/Blueprints/Tiles/Buildings/Building.food_cost` _returnvalue_2) (`/Game/Blueprints/Tiles/Buildings/Building.energy_cost` _returnvalue_2)))
        (if _isenough
          (bind _isenoughap (`/Game/Blueprints/Gamemodes/AnthroGameMode.CheckAP` _asanthro_game_mode 1))
          (if _isenoughap
            (message `/Game/Blueprints/Gameplay/iStatsAndFlows.TrackBuilding` self _returnvalue_2)
            (set `/Game/Blueprints/Tiles/Buildings/Building.owner_player` self _returnvalue_2)
            (`/Game/Blueprints/Tiles/Buildings/Building.Cost` _returnvalue_2)
            (`/Game/Blueprints/Tiles/Buildings/Building.SetBiomeType` _returnvalue_2 (`/Game/Blueprints/Tiles/Biomes/HexTileBasic.BiomeType` HexTileRef) (`PrimitiveComponent.GetMaterial` (`/Game/Blueprints/Tiles/Biomes/HexTileBasic.TileMesh` HexTileRef) 0))
            (`/Game/Blueprints/Tiles/Buildings/Building.CheckBuildingAdjacency` _returnvalue_2)
            (`/Game/Blueprints/Tiles/Buildings/Building.SetSelectableTiles` _returnvalue_2)
            (`|SpawnActorFromClass` "/Game/Blueprints/Gameplay/BuildingExplosion.BuildingExplosion_C" _returnvalue "Undefined" "OverrideRootScale")
            (bind _playertoken (`/Game/Blueprints/Tiles/Buildings/Building.PlayerToken` _returnvalue_2))
            (bind _returnvalue_3 (`KismetMaterialLibrary.CreateDynamicMaterialInstance` (`PrimitiveComponent.GetMaterial` _playertoken 0)))
            (if (`|EnumEquality` (`self.playerNo`) "PN_0")
              (`MaterialInstanceDynamic.SetVectorParameterValue` _returnvalue_3 "BaseColour" (make `LinearColor` 0.0 0.5 0.8 0.9))
              (else
                (`MaterialInstanceDynamic.SetVectorParameterValue` _returnvalue_3 "BaseColour" (make `LinearColor` 0.9 0.2 0.0 0.9))))
            (`PrimitiveComponent.SetMaterial` _playertoken 0 _returnvalue_3)
            (`GameplayStatics.PlaySound2D` "/Game/Sounds/Evan_King_-_20XX_-_84_menu_confirm_2_reverb.Evan_King_-_20XX_-_84_menu_confirm_2_reverb")
            (return true _returnvalue _returnvalue_2)
            (else
              (`self.K2_DestroyActor` _returnvalue_2)))
          (else
            (`self.K2_DestroyActor` _returnvalue_2))))
      (:`CastFailed`
        (`KismetSystemLibrary.PrintString` "CastFailed")
        (return false (struct) null))))
  (`GameplayStatics.PlaySound2D` "/Game/Sounds/Evan_King_-_20XX_-_86_menu_deny_1_reverb.Evan_King_-_20XX_-_86_menu_deny_1_reverb")
  (return false (struct) null))

(fn `CheckResources`
  (params (Money :type "Integer (by ref)") (Food :type "Integer (by ref)") (Energy :type "Integer (by ref)"))
  (returns (isEnough :type Boolean))
  ;[1 1 1] Money
  (if (>= Money 1)
    (if (>= (`self.Money`) Money)
      ;[1 1 1] Food
      (if (>= Food 1) :!label _label
        (if (>= (`self.Food`) Food)
          ;[1 1 1] Energy
          (if (>= Energy 1) :!label _label_2
            (if (>= (`self.Energy`) Energy)
              (return true)
              (else
                _))
            (else
              (return true))))
        (else
          (goto _label_2))))
    (else
      (goto _label)))
  (return false))

(fn `CheckWinConditions`
  (bind _asanthro_game_mode (cast `/Game/Blueprints/Gamemodes/AnthroGameMode` (`GameplayStatics.GetGameMode`)))
  (if (>= (`self.Happiness`) (`/Game/Blueprints/Gamemodes/AnthroGameMode.HappinessGoal` _asanthro_game_mode))
    (bind _asmain_controller (cast `/Game/Blueprints/Gameplay/MainController` (`GameplayStatics.GetPlayerController` 0)))
    (`/Game/Blueprints/Gameplay/MainController.AddNotification` _asmain_controller (`KismetStringLibrary.Concat_StrStr` (`|GetEnumeratorNameAsString` (`self.playerNo`)) " Wins!"))
    (bind _returnvalue (`|CreateWidget` "/Game/Blueprints/UI/Winner.Winner_C"))
    (`UserWidget.AddToViewport` _returnvalue 10)))

(fn `GetBuildingType`
  (params (`BuildingNo.` :type Integer))
  (returns (BuildingType :type "/Game/Blueprints/Tiles/Buildings/Building Class Reference"))
  (return (`KismetArrayLibrary.Array_Get` (`self.SpawnableBuildings`) `BuildingNo.`)))

(fn `GetGeneration`
  (bind _funding (`self.Funding`))
  (set `self.FoodGenerated` _funding)
  (set `self.MoneyGenerated` _funding)
  (set `self.EnergyGenerated` _funding)
  (for _array_element (`self.BuildingsOwned`)
    (bind _asbuilding (cast `/Game/Blueprints/Tiles/Buildings/Building` _array_element))
    (bind _food_generate (`/Game/Blueprints/Tiles/Buildings/Building.food_generate` _asbuilding))
    (bind _output_get (set `self.FoodGenerated` (- (+ _food_generate (`self.FoodGenerated`)) (`/Game/Blueprints/Tiles/Buildings/Building.food_upkeep` _asbuilding))))
    (bind _energy_generate (`/Game/Blueprints/Tiles/Buildings/Building.energy_generate` _asbuilding))
    (bind _output_get_2 (set `self.EnergyGenerated` (- (+ _energy_generate (`self.EnergyGenerated`)) (`/Game/Blueprints/Tiles/Buildings/Building.energy_upkeep` _asbuilding))))
    (bind _money_generate (`/Game/Blueprints/Tiles/Buildings/Building.money_generate` _asbuilding))
    (bind _output_get_3 (set `self.MoneyGenerated` (- (+ _money_generate (`self.MoneyGenerated`)) (`/Game/Blueprints/Tiles/Buildings/Building.money_upkeep` _asbuilding))))
    (bind _biomebonus (`/Game/Blueprints/Tiles/Buildings/Building.BiomeBonus` _asbuilding))
    (bind _biometype (`/Game/Blueprints/Tiles/Biomes/HexTileBasic.BiomeType` _asbuilding))
    (if (`KismetArrayLibrary.Array_Contains` _biomebonus _biometype)
      (if (> _food_generate 0)
        (bind _item (`KismetArrayLibrary.Array_Get` (`/Game/Blueprints/Tiles/Buildings/Building.BiomeBonusEffect` _asbuilding) (`KismetArrayLibrary.Array_Find` _biomebonus _biometype)))
        (set `self.FoodGenerated` (+ _item _output_get)))
      (if (> _energy_generate 0)
        (set `self.EnergyGenerated` (+ _item _output_get_2)))
      (if (> _money_generate 0)
        (set `self.MoneyGenerated` (+ _item _output_get_3))))))

(fn `GetStats`
  (returns (Happiness :type Integer) (Money :type Integer) (Energy :type Integer) (Food :type Integer))
  (return (`self.Happiness`) (`self.Money`) (`self.Energy`) (`self.Food`)))

(fn `UserConstructionScript`)