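; Controller for the hex-tile editor that creates the editor UI and pause menu, tracks the selected tile and fades notifications.
; SaveGame writes editor UI settings, the tile container and fresh turn defaults to slot "Save1".
; LoadGame restores game mode and player stats, then rebuilds the board from saved tiles.
; Non-city-centre buildings get owners and copy biome and material from their base tile via a briefly spawned actor.
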(event `self.ReceiveBeginPlay`
  (bind _returnvalue (`|CreateWidget` "/Game/Blueprints/UI/EditorUI_2016-08-09-21-45-57.EditorUI_C"))
  (set `self.EditorUIRef` _returnvalue)
  (`UserWidget.AddToViewport` _returnvalue 1)
  (bind _returnvalue_2 (`|CreateWidget` "/Game/Blueprints/UI/PauseMenu.PauseMenu_C"))
  (set `self.PauseMenuRef` _returnvalue_2)
  (`UserWidget.AddToViewport` _returnvalue_2 6))

(event `FadeNotification`
  (params (Notification :type "Button Object Reference"))
  (bind (_direction _alphavalues) (`Timeline|FadeTimeline` :!via `PlayFromStart`)
    (:`Update`
      (`Button.SetColorAndOpacity` Notification (`KismetMathLibrary.MakeColor` 0.0 0.0 0.0 _alphavalues)))
    (:`Finished`
      (`PanelWidget.ClearChildren` (`/Game/Blueprints/UI/HUD_Main.TempNotification` (`self.HUDMainRef`)))
      (`/Engine/EditorBlueprintResources/StandardMacros.DecrementInt` (`self.NoOfNotications`)))))

(fn `GetSelectedTile`
  (returns (SelectedTile :type "/Game/Blueprints/Tiles/Biomes/HexTileBasic Object Reference"))
  (return (`self.ActiveTile`)))

(fn `LoadGame`
  (bind _returnvalue (`GameplayStatics.DoesSaveGameExist` "Save1"))
  (if _returnvalue
    (bind _returnvalue_2 (`GameplayStatics.LoadGameFromSlot` "Save1"))
    (bind _asanthro_save_game (cast `/Game/Blueprints/Gameplay/AnthroSaveGame` _returnvalue_2))
    (bind _output_get (set `self.SaveGameState` _asanthro_save_game))
    (bind _asanthro_game_mode (cast `/Game/Blueprints/Gamemodes/AnthroGameMode` (`GameplayStatics.GetGameMode`)))
    (bind _playerstatobjects (`/Game/Blueprints/Gamemodes/AnthroGameMode.PlayerStatObjects` _asanthro_game_mode))
    (bind _item (`KismetArrayLibrary.Array_Get` _playerstatobjects))
    (set `/Game/Blueprints/Gameplay/PlayerStatsMain.Food` (`/Game/Blueprints/Gameplay/AnthroSaveGame.p1Food` _output_get) _item)
    (set `/Game/Blueprints/Gameplay/PlayerStatsMain.Money` (`/Game/Blueprints/Gameplay/AnthroSaveGame.p1Money` _output_get) _item)
    (set `/Game/Blueprints/Gameplay/PlayerStatsMain.Energy` (`/Game/Blueprints/Gameplay/AnthroSaveGame.p1Energy` _output_get) _item)
    (set `/Game/Blueprints/Gameplay/PlayerStatsMain.Happiness` (`/Game/Blueprints/Gameplay/AnthroSaveGame.p1Happiness` _output_get) _item)
    (bind _item_2 (`KismetArrayLibrary.Array_Get` _playerstatobjects 1))
    (set `/Game/Blueprints/Gameplay/PlayerStatsMain.Food` (`/Game/Blueprints/Gameplay/AnthroSaveGame.p2Food` _output_get) _item_2)
    (set `/Game/Blueprints/Gameplay/PlayerStatsMain.Energy` (`/Game/Blueprints/Gameplay/AnthroSaveGame.p2Energy` _output_get) _item_2)
    (set `/Game/Blueprints/Gameplay/PlayerStatsMain.Money` (`/Game/Blueprints/Gameplay/AnthroSaveGame.p2Money` _output_get) _item_2)
    (set `/Game/Blueprints/Gameplay/PlayerStatsMain.Happiness` (`/Game/Blueprints/Gameplay/AnthroSaveGame.p2Happiness` _output_get) _item_2)
    (set `/Game/Blueprints/Gamemodes/AnthroGameMode.activePlayer` (`/Game/Blueprints/Gameplay/AnthroSaveGame.ActivePlayer` _output_get) _asanthro_game_mode)
    (set `/Game/Blueprints/Gamemodes/AnthroGameMode.TurnCount` (`/Game/Blueprints/Gameplay/AnthroSaveGame.TurnNumber` _output_get) _asanthro_game_mode)
    (bind _outactors (`GameplayStatics.GetAllActorsOfClass` "/Game/Blueprints/Tiles/Biomes/HexTileBasic.HexTileBasic_C"))
    (`self.K2_DestroyActor` _outactors)
    (set `/Game/Blueprints/Gamemodes/AnthroGameMode.players` (`/Game/Blueprints/Gameplay/AnthroSaveGame.NumberOfPlayers` _output_get) _asanthro_game_mode)
    (set `/Game/Blueprints/Gamemodes/AnthroGameMode.actionPoints` (`/Game/Blueprints/Gameplay/AnthroSaveGame.APRemaining` _asanthro_save_game) _asanthro_game_mode)
    (bind _tilestorage (`/Game/Blueprints/Gameplay/AnthroSaveGame.TileStorage` _output_get))
    (for _array_element _tilestorage
      (bind (_location _building _id _basetile) (break `/Game/Blueprints/Tiles/TileInfo` _array_element))
      (if (`KismetMathLibrary.ClassIsChildOf` _building "/Game/Blueprints/Tiles/Buildings/Building.Building_C")
        (if (!= _building "/Game/Blueprints/Tiles/Buildings/CityCentre.CityCentre_C")
          (for _array_element_2 (`self.AllBuildings`)
            (if (== _array_element_2 _building)
              (bind _returnvalue_3 (`|SpawnActorFromClass` _array_element_2 _location "Undefined" "OverrideRootScale"))
              ;[1 1 1] Spawn the tile to get the material
              (bind _returnvalue_4 (`|SpawnActorFromClass` _basetile _location "Undefined" "OverrideRootScale"))
              (set `/Game/Blueprints/Tiles/Biomes/HexTileBasic.BiomeType` (`.BiomeType` (defaults `/Game/Blueprints/Gameplay/MainController` _basetile)) _returnvalue_3)
              (`PrimitiveComponent.SetMaterial` (`/Game/Blueprints/Tiles/Biomes/HexTileBasic.TileMesh` _returnvalue_3) 0 (`PrimitiveComponent.GetMaterial` (`/Game/Blueprints/Tiles/Biomes/HexTileBasic.TileMesh` _returnvalue_4) 0))
              (`self.K2_DestroyActor` _returnvalue_4)
              (bind _asanthro_game_mode_2 (cast `/Game/Blueprints/Gamemodes/AnthroGameMode` (`GameplayStatics.GetGameMode`)))
              (if (`|EnumEquality` _id "PN_0")
                (bind _playerstatobjects_2 (`/Game/Blueprints/Gamemodes/AnthroGameMode.PlayerStatObjects` _asanthro_game_mode_2))
                (bind _returnvalue_5 (`KismetMathLibrary.Conv_ByteToInt` _id))
                (bind _item_3 (`KismetArrayLibrary.Array_Get` _playerstatobjects_2 _returnvalue_5))
                (message `/Game/Blueprints/Gameplay/iStatsAndFlows.TrackBuilding` _item_3 _returnvalue_3)
                (set `/Game/Blueprints/Tiles/Buildings/Building.owner_player` _item_3 _returnvalue_3)
                (else
                  (bind _item_4 (`KismetArrayLibrary.Array_Get` _playerstatobjects_2 _returnvalue_5))
                  (message `/Game/Blueprints/Gameplay/iStatsAndFlows.TrackBuilding` _item_4 _returnvalue_3)
                  (set `/Game/Blueprints/Tiles/Buildings/Building.owner_player` _item_4 _returnvalue_3)))))
          (else
            (`|SpawnActorFromClass` _building _location "Undefined" "OverrideRootScale")))
        (else
          (`|SpawnActorFromClass` _building _location "Undefined" "OverrideRootScale"))))
    (bind _asglobal_data (cast `/Game/Blueprints/Gameplay/GlobalData` (`GameplayStatics.GetGameInstance`)))
    (set `/Game/Blueprints/Gameplay/GlobalData.LoadGame?` false _asglobal_data)
    (set `self.TileContainer` _tilestorage)
    (else
      (`KismetSystemLibrary.PrintString` "No save data"))))

(fn `SaveGame`
  (bind _editoruiref (`self.EditorUIRef`))
  (bind _returnvalue (`GameplayStatics.CreateSaveGameObject` "/Game/Blueprints/Gameplay/AnthroSaveGame.AnthroSaveGame_C"))
  (bind _asanthro_save_game (cast `/Game/Blueprints/Gameplay/AnthroSaveGame` _returnvalue))
  (bind _output_get (set `self.SaveGameState` _asanthro_save_game))
  (set `/Game/Blueprints/Gameplay/AnthroSaveGame.p1Energy` (`/Game/Blueprints/UI/EditorUI_2016-08-09-21-45-57.p1energy` _editoruiref) _output_get)
  (set `/Game/Blueprints/Gameplay/AnthroSaveGame.p1Food` (`/Game/Blueprints/UI/EditorUI_2016-08-09-21-45-57.p1food` _editoruiref) _output_get)
  (set `/Game/Blueprints/Gameplay/AnthroSaveGame.p1Money` (`/Game/Blueprints/UI/EditorUI_2016-08-09-21-45-57.p1money` _editoruiref) _output_get)
  (set `/Game/Blueprints/Gameplay/AnthroSaveGame.p1Happiness` 0 _output_get)
  (set `/Game/Blueprints/Gameplay/AnthroSaveGame.p2Energy` (`/Game/Blueprints/UI/EditorUI_2016-08-09-21-45-57.p2energy` _editoruiref) _output_get)
  (set `/Game/Blueprints/Gameplay/AnthroSaveGame.p2Food` (`/Game/Blueprints/UI/EditorUI_2016-08-09-21-45-57.p2food` _editoruiref) _output_get)
  (set `/Game/Blueprints/Gameplay/AnthroSaveGame.p2Money` (`/Game/Blueprints/UI/EditorUI_2016-08-09-21-45-57.p2money` _editoruiref) _output_get)
  (set `/Game/Blueprints/Gameplay/AnthroSaveGame.p2Happiness` 0 _output_get)
  (set `/Game/Blueprints/Gameplay/AnthroSaveGame.TileStorage` (`self.TileContainer`) _output_get)
  (set `/Game/Blueprints/Gameplay/AnthroSaveGame.TurnNumber` 0 _output_get)
  (set `/Game/Blueprints/Gameplay/AnthroSaveGame.ActivePlayer` "PN_0" _output_get)
  (set `/Game/Blueprints/Gameplay/AnthroSaveGame.NumberOfPlayers` (`/Game/Blueprints/UI/EditorUI_2016-08-09-21-45-57.NumberOfPlayers` _editoruiref) _output_get)
  (set `/Game/Blueprints/Gameplay/AnthroSaveGame.APRemaining` 5 _output_get)
  (set `/Game/Blueprints/Gameplay/AnthroSaveGame.TurnLimitValue` (`/Game/Blueprints/UI/EditorUI_2016-08-09-21-45-57.TurnLimit` _editoruiref) _output_get)
  (`GameplayStatics.SaveGameToSlot` (`self.SaveGameState`) "Save1"))

(fn `SetSelectedTile`
  (params (`new tile` :type "/Game/Blueprints/Tiles/Biomes/HexTileBasic Object Reference"))
  (returns (Output :type "/Game/Blueprints/Tiles/Biomes/HexTileBasic Object Reference"))
  (bind _output_get (set `self.ActiveTile` `new tile`))
  (return _output_get))

(fn `UserConstructionScript`)